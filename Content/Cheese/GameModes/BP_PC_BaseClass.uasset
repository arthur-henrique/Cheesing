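; Base player controller that routes player input to the HUD for the collectables screen and pausing.
; BeginPlay fetches and caches the base HUD through a GetBPHUDBaseCLass call with a Success output.
; The C key refreshes the collectables widget from the HUD's inventory and toggles it.
; The Pause_Game action asks the HUD to pause, except in the main menu level, where it only prints a message.
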(event EventBeginPlay
  (bind _asbp_hud_base_class (Utilities|GetBPHUDBaseCLass 1e+01)
    (:Success
      (Variables|Default|SetAs%20BP%20HUD%20Base%20Class _asbp_hud_base_class))))

(event EventTick
  (params (DeltaSeconds :type Float%20%28single-precision%29)))

(event Input|ActionEvents|InputActionPause_Game
  (params (Key :type Key%20Structure :default "None"))
  (:Pressed
    (bind _returnvalue (Game|GetCurrentLevelName true))
    (if (Utilities|Enum|NotEqual(Enum) _returnvalue "L_MainMenu")
      (Default|PausetheGame (Variables|Default|GetAs%20BP%20HUD%20Base%20Class))
      (else
        (Development|PrintString "Cant Pause")))))

(event Input|KeyboardEvents|C
  (params (Key :type Key%20Structure :default "None"))
  (bind _as_bp_hud_base_class (Variables|Default|GetAs%20BP%20HUD%20Base%20Class))
  (:Pressed
    (Default|UpdateInventory (Variables|/Game/Cheese/GameModes/BP_HUD_BaseClass.BP_HUD_BaseClass_C|GetWB_Collectables _as_bp_hud_base_class) (Variables|/Game/Cheese/GameModes/BP_HUD_BaseClass.BP_HUD_BaseClass_C|GetInventory _as_bp_hud_base_class))
    (Default|ToggleCollectables (Variables|Default|GetAs%20BP%20HUD%20Base%20Class))))

(fn ConstructionScript)