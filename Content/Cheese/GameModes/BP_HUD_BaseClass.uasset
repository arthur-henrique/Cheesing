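; Base HUD that owns the game's menu widgets and handles starting, pausing, options, returning to the main menu and quitting.
; BeginPlay adds main menu, pause and options widgets to the viewport, creating a collectables widget inside that same loop.
; Events call functions that switch visibility, input mode, cursor and pause state, or open levels by name.
; ToggleWidget shows or hides one game-menu widget while collapsing the others.
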(event Custom|Toggle_Collectables
  ;[1 1 1] Toggle Collectables Game Menu
  (CallFunction|ToggleWidget (Variables|Default|GetWB_Collectables)))

(event Custom|ResumeGame
  ;[1 1 1] Resume Game from Pause
  (CallFunction|ResumefromPause))

(event Custom|PauseTheGame
  ;[1 1 1] Pause the Game
  (CallFunction|PauseGame))

(event Custom|OpenOptions
  ;[1 1 1] Open options
  (CallFunction|AccessOptionsMenu))

(event Custom|QuitGame
  ;[1 1 1] Quit Game
  (Game|QuitGame 0 "Quit" false))

(event Custom|CloseOptions
  ;[1 1 1] Close Options
  (CallFunction|ReturnfromOptions))

(event Custom|StartGame
  ;[1 1 1] Start Game
  (CallFunction|StarttheGame))

(event Custom|ReturnToMenu
  ;[1 1 1] Return To Menu
  (CallFunction|BacktoMainMenu))

(event EventBeginPlay
  (bind _returnvalue (Game|Player|GetOwningPlayerController))
  (bind _gamemenus_widgetlist (Variables|Default|GetGameMenus_WidgetList))
  (bind _menus_widgetlist (Variables|Default|GetMenus_WidgetList))
  (Input|SetInputModeGameOnly _returnvalue)
  (bind _returnvalue_2 (UserInterface|CreateWidget "/Game/Cheese/HUD/WB_MainMenu.WB_MainMenu_C" _returnvalue))
  (bind _output_get (Variables|Default|SetWB_MainMenu _returnvalue_2))
  (Utilities|Array|Add (Variables|Default|GetMenus_WidgetList) _output_get)
  (bind _returnvalue_3 (UserInterface|CreateWidget "/Game/Cheese/HUD/WB_Pause.WB_Pause_C" (Game|Player|GetOwningPlayerController)))
  (bind _output_get_2 (Variables|Default|SetWB_Pause _returnvalue_3))
  (Utilities|Array|Add (Variables|Default|GetMenus_WidgetList) _output_get_2)
  (bind _returnvalue_4 (UserInterface|CreateWidget "/Game/Cheese/HUD/WB_MainMenuOptions.WB_MainMenuOptions_C" (Game|Player|GetOwningPlayerController)))
  (bind _output_get_3 (Variables|Default|SetWB_MainMenuPause _returnvalue_4))
  (Default|OnStart _output_get_3)
  (Utilities|Array|Add _menus_widgetlist _output_get_3)
  (for _array_element _menus_widgetlist
    (UserInterface|Viewport|AddtoViewport _array_element 0)
    (bind _returnvalue_5 (UserInterface|CreateWidget "/Game/Cheese/HUD/WB_Collectables.WB_Collectables_C"))
    (bind _output_get_4 (Variables|Default|SetWB_Collectables _returnvalue_5))
    (Utilities|Array|Add _gamemenus_widgetlist _output_get_4)
    (for _array_element_2 _gamemenus_widgetlist
      (UserInterface|Viewport|AddtoViewport _array_element_2 0))))

(fn ConstructionScript)

(fn ToggleWidget
  (params (TargetWidget :type User%20Widget%20Object%20Reference))
  (Utilities|IsValid TargetWidget
    (:Is%20Valid
      (Variables|Default|SetWidgetToFocus TargetWidget)
      (for _array_element (Variables|Default|GetGameMenus_WidgetList)
        (Utilities|IsValid _array_element
          (:Is%20Valid
            (if (== (Variables|Default|GetWidgetToFocus) _array_element)
              (if (Widget|IsVisible (Variables|Default|GetWidgetToFocus))
                (CallFunction|FocusGame)
                (else
                  (CallFunction|FocusWidget)))
              (elif (Widget|IsVisible _array_element)
                (Widget|SetVisibility _array_element "Collapsed")))))))))

(fn FocusGame
  (bind _returnvalue (Game|Player|GetOwningPlayerController))
  (Widget|SetVisibility (Variables|Default|GetWidgetToFocus) "Collapsed")
  (Input|SetInputModeGameOnly _returnvalue)
  (Variables|/Script/Engine.PlayerController|SetbShowMouseCursor _returnvalue false))

(fn FocusWidget
  (bind _returnvalue (Game|Player|GetOwningPlayerController))
  (Widget|SetVisibility (Variables|Default|GetWidgetToFocus) "SelfHitTestInvisible")
  (Input|SetInputModeGameandUI _returnvalue (Variables|Default|GetWidgetToFocus) "DoNotLock" true)
  (Variables|/Script/Engine.PlayerController|SetbShowMouseCursor _returnvalue true))

(fn ResumefromPause
  (bind _returnvalue (Game|Player|GetOwningPlayerController))
  (Widget|SetVisibility (Variables|Default|GetWB_Pause) "Collapsed")
  (Game|SetGamePaused false)
  (Input|SetInputModeGameOnly _returnvalue)
  (Variables|/Script/Engine.PlayerController|SetbShowMouseCursor _returnvalue false))

(fn PauseGame
  (bind _returnvalue (Game|Player|GetOwningPlayerController))
  (bind _wb_pause (Variables|Default|GetWB_Pause))
  (Utilities|FlowControl|Sequence
    (:then_0
      (for _array_element (Variables|Default|GetGameMenus_WidgetList)
        (if (Widget|IsVisible _array_element)
          (Widget|SetVisibility _array_element "Collapsed"))))
    (:then_1
      (if (Game|IsGamePaused)
        (Widget|SetVisibility _wb_pause "Collapsed")
        (Input|SetInputModeGameOnly _returnvalue)
        (Variables|/Script/Engine.PlayerController|SetbShowMouseCursor _returnvalue false)
        (Game|SetGamePaused false)
        (else
          (Widget|SetVisibility _wb_pause "Visible")
          (Game|SetGamePaused true)
          (Variables|/Script/Engine.PlayerController|SetbShowMouseCursor _returnvalue true)
          (Input|SetInputModeGameandUI (Game|Player|GetOwningPlayerController) (Variables|Default|GetWB_Pause) "LockInFullscreen" false))))))

(fn AccessOptionsMenu
  (Widget|SetVisibility (Variables|Default|GetWB_MainMenuPause) "Visible"))

(fn ReturnfromOptions
  (Widget|SetVisibility (Variables|Default|GetWB_MainMenuPause) "Collapsed"))

(fn StarttheGame
  (bind _returnvalue (Game|Player|GetOwningPlayerController))
  (Widget|SetVisibility (Variables|Default|GetWB_MainMenu) "Collapsed")
  (Input|SetInputModeGameOnly _returnvalue)
  (Variables|/Script/Engine.PlayerController|SetbShowMouseCursor _returnvalue false)
  (Game|OpenLevel(byName) "L_CharacterTesting")
  (Game|SetGamePaused false))

(fn BacktoMainMenu
  (for _array_element (Variables|Default|GetGameMenus_WidgetList)
    (Widget|SetVisibility _array_element "Collapsed"))
  (for _array_element_2 (Variables|Default|GetMenus_WidgetList)
    (Widget|SetVisibility _array_element_2 "Collapsed"))
  (Game|OpenLevel(byName) "L_MainMenu")
  (Widget|SetVisibility (Variables|Default|GetWB_MainMenu) "Visible"))