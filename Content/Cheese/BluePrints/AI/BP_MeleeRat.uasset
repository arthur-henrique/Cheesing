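; BP_MeleeRat is a melee rat enemy that seeks the player and can be bounced on.
; Overlaps on its Detection volume set PlayerDetected and start or stop seeking ThirdPersonCharacter, while any overlap on BounceRadius launches the player upward.
; The construction script assigns its detection, attack range and bounce components to radius variables.
; The seek and launch functions are only called here, and no attack logic appears in this graph.
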(event OnComponentBeginOverlap(BounceRadius)
  (params (OverlappedComponent :type Primitive%20Component%20Object%20Reference) (OtherActor :type Actor%20Object%20Reference) (OtherComp :type Primitive%20Component%20Object%20Reference) (OtherBodyIndex :type Integer) (bFromSweep :type Boolean) (SweepResult :type Hit%20Result%20Structure%20%28by%20ref%29))
  (Class|MeleeRat|LaunchPlayerUp))

(event OnComponentBeginOverlap(Detection)
  (params (OverlappedComponent :type Primitive%20Component%20Object%20Reference) (OtherActor :type Actor%20Object%20Reference) (OtherComp :type Primitive%20Component%20Object%20Reference) (OtherBodyIndex :type Integer) (bFromSweep :type Boolean) (SweepResult :type Hit%20Result%20Structure%20%28by%20ref%29))
  (if (== (Utilities|GetClass OtherActor) "/Game/ThirdPersonCPP/Blueprints/ThirdPersonCharacter.ThirdPersonCharacter_C")
    (Variables|Default|SetplayerDetected true)
    (Class|MeleeRat|SeekPlayer)))

(event OnComponentEndOverlap(Detection)
  (params (OverlappedComponent :type Primitive%20Component%20Object%20Reference) (OtherActor :type Actor%20Object%20Reference) (OtherComp :type Primitive%20Component%20Object%20Reference) (OtherBodyIndex :type Integer))
  (if (== (Utilities|GetClass OtherActor) "/Game/ThirdPersonCPP/Blueprints/ThirdPersonCharacter.ThirdPersonCharacter_C")
    (Variables|Default|SetplayerDetected false)
    (Class|MeleeRat|StopSeekingPlayer)))

(event EventBeginPlay
  (bind _returnvalue (Actor|GetActorOfClass "/Game/ThirdPersonCPP/Blueprints/ThirdPersonCharacter.ThirdPersonCharacter_C"))
  (Variables|Default|SetplayerRef _returnvalue))

(event Collision|EventActorBeginOverlap
  (params (OtherActor :type Actor%20Object%20Reference)))

(event EventTick
  (params (DeltaSeconds :type Float%20%28single-precision%29)))

(fn ConstructionScript
  (Variables|Default|SetdetectionRadius (Variables|Default|GetDetection))
  (Variables|Default|SetattackDetectionRadius (Variables|Default|GetAttackRange))
  (Variables|Default|SetheadRadius (Variables|Default|GetBounce%20Radius)))