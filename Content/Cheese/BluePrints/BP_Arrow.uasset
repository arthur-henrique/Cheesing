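; BP_Arrow is an arrow actor that moves up and down along world Z in a continuous loop.
; Tick accumulates elapsed time, raising the actor at Speed for three seconds, then lowering it at the same rate until the timer passes six seconds and resets.
; Movement uses delta-time-scaled SetActorLocation offsets from the current position without sweeping, rather than a stored origin or timeline.
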(event EventBeginPlay)

(event Collision|EventActorBeginOverlap
  (params (OtherActor :type Actor%20Object%20Reference)))

(event EventTick
  (params (DeltaSeconds :type Float%20%28single-precision%29))
  (bind _returnvalue (Transformation|GetActorLocation))
  (bind _returnvalue_2 (Transformation|GetActorLocation))
  (bind _speed (Variables|Default|Getspeed))
  (bind (_x _y _z) (Math|Vector|BreakVector _returnvalue_2))
  (bind (_x_2 _y_2 _z_2) (Math|Vector|BreakVector _returnvalue))
  (bind _returnvalue_3 (* _speed DeltaSeconds))
  (Variables|Default|SettimePassed (+ DeltaSeconds (Variables|Default|GettimePassed)))
  (if (< (Variables|Default|GettimePassed) 3.0)
    (Transformation|SetActorLocation (Math|Vector|MakeVector _x _y (+ _z _returnvalue_3)) false false)
    (else
      (Transformation|SetActorLocation (Math|Vector|MakeVector _x_2 _y_2 (+ _z_2 (* -1 _returnvalue_3))) false false)
      (if (> (Variables|Default|GettimePassed) 6.0)
        (Variables|Default|SettimePassed 0.0)))))

(fn ConstructionScript)