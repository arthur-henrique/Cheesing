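; BP_Checkpoint is a checkpoint actor that records the player's latest checkpoint location.
; On BeginPlay it caches a reference to BP_CheesingGameInstance.
; When an actor whose class is exactly ThirdPersonCharacter begins overlapping its Box, it writes its own location to the game instance's LastCheckpoint.
; Each such overlap also spawns a confetti emitter attached to its Confetti component, with no guard against retriggering.
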(event OnComponentBeginOverlap(Box)
  (params (OverlappedComponent :type Primitive%20Component%20Object%20Reference) (OtherActor :type Actor%20Object%20Reference) (OtherComp :type Primitive%20Component%20Object%20Reference) (OtherBodyIndex :type Integer) (bFromSweep :type Boolean) (SweepResult :type Hit%20Result%20Structure%20%28by%20ref%29))
  (if (== (Utilities|GetClass OtherActor) "/Game/ThirdPersonCPP/Blueprints/ThirdPersonCharacter.ThirdPersonCharacter_C")
    (Variables|/Script/Cheesing.CheesingGameInstance|SetlastCheckpoint (Variables|Default|GetinstanceRef) (Transformation|GetActorLocation))
    (Effects|SpawnEmitterAttached "/Game/Cheese/VFX/Niagara/Confetti.Confetti" (Variables|Default|GetConfetti) "None")))

(event EventBeginPlay
  (bind _asbp_cheesing_game_instance (Utilities|Casting|CastToBP_CheesingGameInstance (Game|GetGameInstance)))
  (Variables|Default|SetinstanceRef _asbp_cheesing_game_instance))

(fn ConstructionScript)