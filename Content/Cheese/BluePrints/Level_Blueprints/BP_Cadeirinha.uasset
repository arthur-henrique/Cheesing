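; BP_Cadeirinha is a level actor ("little chair") that animates its own transform for a short time when activated.
; OnActivation sets the Animating flag, then clears it after a five-second delay.
; While flagged, Tick eases rotation toward a hard-coded target using DeltaSeconds as lerp alpha and sets relative location to the origin.
; A location lerp toward a fixed point and direct set-transform nodes remain unconnected.
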(event EventBeginPlay)

(event Collision|EventActorBeginOverlap
  (params (OtherActor :type Actor%20Object%20Reference)))

(event EventTick
  (params (DeltaSeconds :type Float%20%28single-precision%29))
  (if (Variables|Default|GetAnimating)
    (Transformation|SetActorRelativeRotation (Math|Rotator|Lerp(Rotator) (Transformation|GetActorRotation) "13.089899,27.364363,52.353561" DeltaSeconds))
    (Transformation|SetActorRelativeLocation "0, 0, 0")))

(event EventOnActivation
  (Variables|Default|SetAnimating true)
  (Utilities|FlowControl|Delay 5.0)
  (Variables|Default|SetAnimating false))

(fn ConstructionScript)