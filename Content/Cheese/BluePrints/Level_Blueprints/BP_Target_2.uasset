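; BP_Target_2 is a hittable level target that rotates when hit and then removes the referenced FogaoDamage actor.
; OnHit turns on the Animating flag, waits through a short delay, then clears the flag and destroys FogaoDamage.
; While the flag is set, Tick eases the target toward a fixed rotation using LerpRotator with delta time as alpha.
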(event EventTick
  (params (DeltaSeconds :type Float%20%28single-precision%29))
  (if (Variables|Default|Getanimating)
    (Transformation|SetActorRotation (Math|Rotator|Lerp(Rotator) (Transformation|GetActorRotation) "270.000000, 0, 0" DeltaSeconds))))

(event EventOnHit
  (Variables|Default|Setanimating true)
  (Utilities|FlowControl|Delay 2.0)
  (Variables|Default|Setanimating false)
  (Actor|DestroyActor (Variables|Default|GetfogaoDamage)))

(fn ConstructionScript)