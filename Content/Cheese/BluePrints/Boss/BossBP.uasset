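; Boss actor that fights the player with aimed projectiles at range and directional melee strikes up close, using nested overlap volumes.
; The outer Sphere starts and stops a Delay-driven firing loop that launches SimpleProjectile toward the player, while InnerSphere pauses shooting and arms melee.
; Front, right and left zones trigger a delayed MeleeImpact spawn at the matching point, followed by a cooldown.
; Boolean flags track range, direction and the Shooting and Attacking states.
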(event OnComponentBeginOverlap(Sphere)
  (params (OverlappedComponent :type Primitive%20Component%20Object%20Reference) (OtherActor :type Actor%20Object%20Reference) (OtherComp :type Primitive%20Component%20Object%20Reference) (OtherBodyIndex :type Integer) (bFromSweep :type Boolean) (SweepResult :type Hit%20Result%20Structure%20%28by%20ref%29))
  ;[1 1 1] No Alcance Total
  (if (== OtherActor (Game|GetPlayerCharacter 0))
    (CallFunction|Activate)
    (Variables|Default|SetTooClose false)))

(event OnComponentEndOverlap(Sphere)
  (params (OverlappedComponent :type Primitive%20Component%20Object%20Reference) (OtherActor :type Actor%20Object%20Reference) (OtherComp :type Primitive%20Component%20Object%20Reference) (OtherBodyIndex :type Integer))
  (if (== OtherActor (Game|GetPlayerCharacter 0))
    (CallFunction|Deactivate)))

(event OnComponentBeginOverlap(FrontAttack)
  (params (OverlappedComponent :type Primitive%20Component%20Object%20Reference) (OtherActor :type Actor%20Object%20Reference) (OtherComp :type Primitive%20Component%20Object%20Reference) (OtherBodyIndex :type Integer) (bFromSweep :type Boolean) (SweepResult :type Hit%20Result%20Structure%20%28by%20ref%29))
  ;[1 1 1] No Alcance do Ataque Frente
  (if (== OtherActor (Game|GetPlayerCharacter 0))
    (Variables|Default|SetCanShoot false)
    (Variables|Default|SetTooClose true)
    (Variables|Default|SetFrente true)
    (Variables|Default|SetDireita false)
    (Variables|Default|SetEsquerda false)
    (CallFunction|Ataque)))

(event OnComponentBeginOverlap(InnerSphere)
  (params (OverlappedComponent :type Primitive%20Component%20Object%20Reference) (OtherActor :type Actor%20Object%20Reference) (OtherComp :type Primitive%20Component%20Object%20Reference) (OtherBodyIndex :type Integer) (bFromSweep :type Boolean) (SweepResult :type Hit%20Result%20Structure%20%28by%20ref%29))
  (if (== OtherActor (Game|GetPlayerCharacter 0))
    (Variables|Default|SetCanShoot false)
    (Variables|Default|SetTooClose true)
    (Variables|Default|SetCanAttack true)))

(event OnComponentBeginOverlap(RightAttack)
  (params (OverlappedComponent :type Primitive%20Component%20Object%20Reference) (OtherActor :type Actor%20Object%20Reference) (OtherComp :type Primitive%20Component%20Object%20Reference) (OtherBodyIndex :type Integer) (bFromSweep :type Boolean) (SweepResult :type Hit%20Result%20Structure%20%28by%20ref%29))
  ;[1 1 1] No Alcance Ataque Direito
  (if (== OtherActor (Game|GetPlayerCharacter 0))
    (Variables|Default|SetCanShoot false)
    (Variables|Default|SetTooClose true)
    (Variables|Default|SetFrente false)
    (Variables|Default|SetDireita true)
    (Variables|Default|SetEsquerda false)
    (CallFunction|Ataque)))

(event OnComponentBeginOverlap(LeftAttack)
  (params (OverlappedComponent :type Primitive%20Component%20Object%20Reference) (OtherActor :type Actor%20Object%20Reference) (OtherComp :type Primitive%20Component%20Object%20Reference) (OtherBodyIndex :type Integer) (bFromSweep :type Boolean) (SweepResult :type Hit%20Result%20Structure%20%28by%20ref%29))
  ;[1 1 1] No Alcance Ataque Esquerdo
  (if (== OtherActor (Game|GetPlayerCharacter 0))
    (Variables|Default|SetCanShoot false)
    (Variables|Default|SetTooClose true)
    (Variables|Default|SetFrente false)
    (Variables|Default|SetDireita false)
    (Variables|Default|SetEsquerda true)
    (CallFunction|Ataque)))

(event OnComponentEndOverlap(InnerSphere)
  (params (OverlappedComponent :type Primitive%20Component%20Object%20Reference) (OtherActor :type Actor%20Object%20Reference) (OtherComp :type Primitive%20Component%20Object%20Reference) (OtherBodyIndex :type Integer))
  (if (== OtherActor (Game|GetPlayerCharacter 0))
    (CallFunction|Activate)
    (Variables|Default|SetTooClose false)
    (Variables|Default|SetCanAttack false)))

(event Custom|Activate
  (bind _spawnpoint (Variables|Default|GetSpawnPoint))
  (bind _returnvalue (Transformation|GetWorldTransform _spawnpoint))
  (Variables|Default|SetCanShoot true)
  (if (Math|Boolean|Equal(Boolean) (Variables|Default|GetCanShoot) true) :!label _label
    (Utilities|FlowControl|Delay 0.5)
    (if (Math|Boolean|Equal(Boolean) (Variables|Default|GetTooClose) true)
      (goto _label)
      (else
        (Variables|Default|SetShooting true)
        (Utilities|FlowControl|Delay 1.4)
        (bind _returnvalue_2 (Game|SpawnActorfromClass "/Game/Cheese/BluePrints/Boss/SimpleProjectile.SimpleProjectile_C" (Math|Transform|MakeTransform (.location _returnvalue) (.rotation _returnvalue) "1,1,1") "Undefined" 0 0))
        (Physics|SetPhysicsLinearVelocity (Variables|/Game/Cheese/BluePrints/Boss/SimpleProjectile.SimpleProjectile_C|GetStaticMesh _returnvalue_2) (* (Math|Vector|GetUnitDirection(Vector) (Transformation|GetWorldLocation (Variables|Default|GetSpawnPoint)) (+ (Transformation|GetActorLocation (Game|GetPlayerCharacter 0)) "0, 0,75.000000")) (Variables|Default|GetProjectileSpeed)) false "None")
        (Variables|Default|SetShooting false)
        (goto _label)))))

(event Custom|Deactivate
  (Variables|Default|SetCanShoot false))

(event Custom|Ataque
  (bind _meleespawnpoint (Variables|Default|GetMeleeSpawnPoint))
  (bind _meleespawnpointright (Variables|Default|GetMeleeSpawnPointRight))
  (bind _meleespawnpointleft (Variables|Default|GetMeleeSpawnPointLeft))
  (bind _returnvalue (Transformation|GetWorldTransform _meleespawnpointleft))
  (bind _returnvalue_2 (Transformation|GetWorldTransform _meleespawnpoint))
  (bind _returnvalue_3 (Transformation|GetWorldTransform _meleespawnpointright))
  (if (Math|Boolean|Equal(Boolean) (Variables|Default|GetCanAttack) true)
    (Variables|Default|SetAttacking true)
    (Variables|Default|SetCanAttack false)
    (Utilities|FlowControl|Delay 0.5)
    (if (Math|Boolean|Equal(Boolean) (Variables|Default|GetFrente) true)
      (Utilities|FlowControl|Delay 0.7)
      (Game|SpawnActorfromClass "/Game/Cheese/BluePrints/Boss/MeleeImpact.MeleeImpact_C" (Math|Transform|MakeTransform (.location _returnvalue_2) (.rotation _returnvalue_2) "1,1,1") "Undefined" 0 0)
      (Variables|Default|SetAttacking false :!label _label)
      (Variables|Default|SetFrente false)
      (Variables|Default|SetDireita false)
      (Variables|Default|SetEsquerda false)
      (CallFunction|Deactivate)
      (Utilities|FlowControl|Delay 2.0)
      (Variables|Default|SetCanAttack true)
      (elif (Math|Boolean|Equal(Boolean) (Variables|Default|GetDireita) true)
        (Utilities|FlowControl|Delay 0.7)
        (Game|SpawnActorfromClass "/Game/Cheese/BluePrints/Boss/MeleeImpact.MeleeImpact_C" (Math|Transform|MakeTransform (.location _returnvalue_3) (.rotation _returnvalue_3) "1,1,1") "Undefined" 0 0)
        (goto _label)
        (elif (Math|Boolean|Equal(Boolean) (Variables|Default|GetEsquerda) true)
          (Utilities|FlowControl|Delay 0.7)
          (Game|SpawnActorfromClass "/Game/Cheese/BluePrints/Boss/MeleeImpact.MeleeImpact_C" (Math|Transform|MakeTransform (.location _returnvalue) (.rotation _returnvalue) "1,1,1") "Undefined" 0 0)
          (goto _label))))))

(fn ConstructionScript)