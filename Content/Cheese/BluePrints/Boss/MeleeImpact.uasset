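; Short-lived melee impact actor, filed with the boss Blueprints, that knocks characters away from its location.
; Characters that begin overlapping its sphere are launched along the flattened, normalized direction from the actor's root plus a straight-up vector, scaled by XplosionForce and added to their current velocity.
; The sphere is destroyed shortly after BeginPlay, so the push only happens in a brief window after spawn.
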(event OnComponentBeginOverlap(Sphere)
  (params (OverlappedComponent :type Primitive%20Component%20Object%20Reference) (OtherActor :type Actor%20Object%20Reference) (OtherComp :type Primitive%20Component%20Object%20Reference) (OtherBodyIndex :type Integer) (bFromSweep :type Boolean) (SweepResult :type Hit%20Result%20Structure%20%28by%20ref%29))
  (bind _ascharacter (Utilities|Casting|CastToCharacter OtherActor))
  (Character|LaunchCharacter _ascharacter (* (+ (Math|Vector|Normalize (Math|Vector|MakeVector (.x (Math|Vector|GetUnitDirection(Vector) (Transformation|GetWorldLocation (Variables|Default|GetDefaultSceneRoot)) (Transformation|GetActorLocation _ascharacter))) (.y (Math|Vector|GetUnitDirection(Vector) (Transformation|GetWorldLocation (Variables|Default|GetDefaultSceneRoot)) (Transformation|GetActorLocation _ascharacter))) 0.0)) "0, 0,1.000000") (Variables|Default|GetXplosionForce)) false false))

(event EventBeginPlay
  (Utilities|FlowControl|Delay 0.1)
  (Components|DestroyComponent (Variables|Default|GetSphere)))

(fn ConstructionScript)